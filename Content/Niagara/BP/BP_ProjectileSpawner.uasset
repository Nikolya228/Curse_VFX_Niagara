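; Spawner actor that repeatedly fires a configurable Niagara VFX projectile, starting on BeginPlay and repeating on a looping timer.
; Each cycle spawns a non-looping BP_BasicVFXHitImpact as the muzzle flash, then after a delay spawns a BP_ProjectileMasterComponent actor.
; It passes the projectile its effects, impact offset and destroy delay, and sets its velocity along X.
; Spawn points add unrotated offsets to the actor location, ignoring the spawner's facing.
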(event `self.ReceiveBeginPlay`
  (`self.SpawnVFX`)
  (`KismetSystemLibrary.K2_SetTimerDelegate` (delegate `SpawnVFX`) (`self.TimerSpawnVFX`) true))

(event `SpawnVFX`
  (`|ExecutionSequence`
    (:`then_0`
      (bind _returnvalue (`|SpawnActorFromClass` "/Game/Niagara/BP/BP_BasicVFXHitImpact.BP_BasicVFXHitImpact_C" (`KismetMathLibrary.MakeTransform` (+ (`self.K2_GetActorLocation`) (`self.Hit Impact Muzzle Offset`))) "Undefined" "MultiplyWithRoot" null null))
      (set `/Game/Niagara/BP/BP_BasicVFXHitImpact.IsLoop` false _returnvalue)
      (set `/Game/Niagara/BP/BP_BasicVFXHitImpact.System Template` (`self.Muzzle VFX`) _returnvalue))
    (:`then_1`
      (`KismetSystemLibrary.Delay` (`self.DelayBeforeProjectile`))
      (bind _returnvalue_2 (`|SpawnActorFromClass` "/Game/Niagara/BP/BP_ProjectileMasterComponent.BP_ProjectileMasterComponent_C" (`KismetMathLibrary.MakeTransform` (+ (`self.K2_GetActorLocation`) (`self.ProjectileOffset`))) "Undefined" "MultiplyWithRoot" null null))
      (set `self.ProjectileVFX` _returnvalue_2)
      (`|ExecutionSequence`
        (:`then_0`
          ;[1 1 1] Set Spawn VFX Projectile
          (set `/Game/Niagara/BP/BP_ProjectileMasterComponent.MuzzleVFX` (`self.Muzzle VFX`) (`self.ProjectileVFX`))
          (`NiagaraComponent.SetAsset` (`/Game/Niagara/BP/BP_ProjectileMasterComponent.NiagaraVFXComponent` (`self.ProjectileVFX`)) (`self.MainProjectile`) true)
          (set `/Game/Niagara/BP/BP_ProjectileMasterComponent.HitImpact` (`self.Hit Impact`) (`self.ProjectileVFX`)))
        (:`then_1`
          ;[1 1 1] Set Projectile Speed
          (set `MovementComponent.Velocity` (* (`self.SpeedProjectile`) (1.0 0.0 0.0)) (`/Game/Niagara/BP/BP_ProjectileMasterComponent.ProjectileMovement` (`self.ProjectileVFX`))))
        (:`then_2`
          (set `/Game/Niagara/BP/BP_ProjectileMasterComponent.Hit Impact Muzzle Offset` (`self.Hit Impact Muzzle Offset`) (`self.ProjectileVFX`))
          (set `/Game/Niagara/BP/BP_ProjectileMasterComponent.DelayBeforeDestroyActor` (`self.Delay Before Destroy Actor`) (`self.ProjectileVFX`)))))))

(fn `UserConstructionScript`)