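; Base projectile actor for Niagara VFX that moves with a projectile movement component and reacts to hitting blocking volumes.
; On box overlap with a BlockingVolume, it stops movement, sets the Niagara kill-particles flag and spawns the impact system at an offset from its location.
; It destroys itself after a configurable delay.
; The muzzle VFX spawn is disconnected, and BeginPlay only runs a short delay.
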(event `self.ReceiveBeginPlay`
  (`KismetSystemLibrary.Delay` 0.05))

(event `self.BoxColisionVFX.OnComponentBeginOverlap`
  (params (OverlappedComponent :type "PrimitiveComponent Object Reference") (OtherActor :type "Actor Object Reference") (OtherComp :type "PrimitiveComponent Object Reference") (OtherBodyIndex :type Integer) (bFromSweep :type Boolean) (SweepResult :type "HitResult Structure (by ref)"))
  (cast `BlockingVolume` OtherActor)
  (`MovementComponent.StopMovementImmediately` (`self.ProjectileMovement`))
  (`NiagaraComponent.SetVariableBool` (`self.NiagaraVFXComponent`) "ShouldKillParticles" true)
  (`self.SpawnVFX` (`self.HitImpact`) (`self.Hit Impact Muzzle Offset`))
  (`KismetSystemLibrary.Delay` (`self.DelayBeforeDestroyActor`))
  (`self.K2_DestroyActor`))

(fn `SpawnVFX`
  (params (NiagaraVFX :type "NiagaraSystem Object Reference") (HitImpactMuzzleOffset :type "Vector Structure"))
  (`NiagaraFunctionLibrary.SpawnSystemAtLocation` NiagaraVFX (+ (`self.K2_GetActorLocation`) HitImpactMuzzleOffset)))

(fn `UserConstructionScript`)