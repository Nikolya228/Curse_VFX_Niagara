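; BP_DissolveSK is a Blueprint that dissolves a Manny skeletal mesh when a DefaultPawn enters its box trigger.
; On overlap it creates dynamic instances of two dissolve materials, assigns them to both mesh slots and attaches the NS_BPDissolve Niagara effect.
; The DissolveAmount timeline drives the matching scalar parameter on both instances, playing from start on entry and reversing on exit.
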(event `self.Box.OnComponentBeginOverlap`
  (params (OverlappedComponent :type "PrimitiveComponent Object Reference") (OtherActor :type "Actor Object Reference") (OtherComp :type "PrimitiveComponent Object Reference") (OtherBodyIndex :type Integer) (bFromSweep :type Boolean) (SweepResult :type "HitResult Structure (by ref)"))
  (cast `DefaultPawn` OtherActor)
  (`|ExecutionSequence`
    (:`then_0`
      (bind _returnvalue (`KismetMaterialLibrary.CreateDynamicMaterialInstance` "/Game/Niagara/CustomNiagara/DissolveSK/BPDissolve/MI_Manny_01_BPDissovle.MI_Manny_01_BPDissovle"))
      (set `self.Created_DY_MI_Manny_01` _returnvalue)
      (bind _returnvalue_2 (`KismetMaterialLibrary.CreateDynamicMaterialInstance` "/Game/Niagara/CustomNiagara/DissolveSK/BPDissolve/MI_Manny_02_BPDissolve.MI_Manny_02_BPDissolve"))
      (set `self.Created_DY_MI_Manny_02` _returnvalue_2))
    (:`then_1`
      (`PrimitiveComponent.SetMaterial` (`self.SkeletalMesh`) 0 (`self.Created_DY_MI_Manny_01`))
      (`PrimitiveComponent.SetMaterial` (`self.SkeletalMesh`) 1 (`self.Created_DY_MI_Manny_02`)))
    (:`then_2`
      (bind (_direction _changedissolveamount) (`Timeline|DissolveAmount` :!via `PlayFromStart` :!label _label)
        (:`Update`
          (`MaterialInstanceDynamic.SetScalarParameterValue` (`self.Created_DY_MI_Manny_01`) "DissolveAmount" _changedissolveamount)
          (`MaterialInstanceDynamic.SetScalarParameterValue` (`self.Created_DY_MI_Manny_02`) "DissolveAmount" _changedissolveamount))))
    (:`then_3`
      (`NiagaraFunctionLibrary.SpawnSystemAttached` "/Game/Niagara/CustomNiagara/DissolveSK/NS_BPDissolve.NS_BPDissolve" (`self.SkeletalMesh`) "None" (0.0 0.0 0.0) (struct) "SnapToTarget"))))

(event `self.Box.OnComponentEndOverlap`
  (params (OverlappedComponent :type "PrimitiveComponent Object Reference") (OtherActor :type "Actor Object Reference") (OtherComp :type "PrimitiveComponent Object Reference") (OtherBodyIndex :type Integer))
  (cast `DefaultPawn` OtherActor)
  (goto _label :!via `Reverse`))

(fn `UserConstructionScript`)